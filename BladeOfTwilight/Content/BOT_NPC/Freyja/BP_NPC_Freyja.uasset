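; BP_NPC_Freyja is the Blueprint for the Freyja NPC character, linking its movement to its animation.
; On BeginPlay it casts the mesh's anim instance to AnimBP_NPC_Freyja and caches the reference.
; Each Tick it pushes the horizontal speed from CharacterMovement velocity into the AnimBP's MoveSpeed, without a validity check on that reference.
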(event EventBeginPlay
  (|CallParentFunction)
  (bind _asanim_bp_npc_freyja (Utilities|Casting|CastToAnimBP_NPC_Freyja (Components|SkeletalMesh|GetAnimInstance (Variables|Character|GetMesh))))
  (Variables|Default|SetAnimBP _asanim_bp_npc_freyja))

(event Collision|EventActorBeginOverlap
  (params (OtherActor :type Actor%20Object%20Reference))
  (|CallParentFunction OtherActor) ; This node is disabled and will not be called.\nDrag off pins to build functionality.
)

(event EventTick
  (params (DeltaSeconds :type Float%20%28single-precision%29))
  (|CallParentFunction DeltaSeconds)
  (Variables|/Game/BOT_AnimBP/NPC/Freyja/AnimBP_NPC_Freyja.AnimBP_NPC_Freyja_C|SetMoveSpeed (Variables|Default|GetAnimBP) (Math|Vector|VectorLengthXY (Variables|/Script/Engine.MovementComponent|GetVelocity (Variables|Character|GetCharacterMovement)))))

(fn ConstructionScript
  (|CallParentFunction))