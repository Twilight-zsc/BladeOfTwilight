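; Base Blueprint for BOT characters, providing shared input-math, weapon-collider and damage helper functions.
; SquareToCircle remaps a 2D vector from square to circular range using the elliptical grid formula.
; SetWeaponCollider resizes and offsets the left and right weapon boxes from per-socket collider data, skipping invalid components.
; TryApplyDamage is a stub that always returns false, and the construction script is empty.
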(fn ConstructionScript)

(fn SquaretoCircle
  (params (InputVec :type Vector%202D%20Structure))
  (bind (_x _y) (Math|Vector2D|BreakVector2D InputVec))
  (return (Math|Vector2D|MakeVector2D (* _x (Math|Float|Sqrt (- 1.0 (* (* _y _y) 0.5)))) (* _y (Math|Float|Sqrt (- 1.0 (* (* _x _x) 0.5)))))))

(fn SetWeaponCollider
  (params (WeaponColliders :type Array%20of%20Weapon%20Collider%20Info%20Structures) (Weapon_L :type Box%20Component%20Object%20Reference) (Weapon_R :type Box%20Component%20Object%20Reference))
  (for _array_element WeaponColliders
    (switch Utilities|FlowControl|Switch|SwitchonWeaponSocket (.WeaponSocketType (Utilities|Struct|BreakWeaponColliderInfo _array_element))
      (:NewEnumerator0
        (Utilities|IsValid Weapon_L
          (:Is%20Valid
            (Components|Box|SetBoxExtent Weapon_L (.BoxExtent (Utilities|Struct|BreakWeaponColliderInfo _array_element)) true)
            (Transformation|SetRelativeLocation Weapon_L (.BoxOffset (Utilities|Struct|BreakWeaponColliderInfo _array_element)) false false))))
      (:NewEnumerator1
        (Utilities|IsValid Weapon_R
          (:Is%20Valid
            (Components|Box|SetBoxExtent Weapon_R (.BoxExtent (Utilities|Struct|BreakWeaponColliderInfo _array_element)) true)
            (Transformation|SetRelativeLocation Weapon_R (.BoxOffset (Utilities|Struct|BreakWeaponColliderInfo _array_element)) false false)))))))

(fn TryApplyDamage
  (params (DamageVar :type Integer))
  (return false))