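; BPC_HitboxHandle is a component that registers box colliders as hitboxes and switches them on or off by name.
; AddHitbox stores each collider in a map keyed by its object name.
; EnableHitbox and DisableHitbox look up a list of names and toggle Generate Overlap Events on each match.
; An unknown name prints a Chinese warning to check whether the hitbox was registered in the handle.
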(event Custom|AddHitbox
  (params (BoxColliders :type Array%20of%20Box%20Component%20Object%20References))
  (for _array_element BoxColliders
    (Utilities|Map|Add (Variables|Default|GetHitboxs) (Utilities|GetObjectName _array_element) _array_element)))

(event Custom|DisableHitbox
  (params (HitboxNames :type Array%20of%20Strings))
  (for _array_element HitboxNames
    (if (.ReturnValue (Utilities|Map|Find (Variables|Default|GetHitboxs) _array_element))
      (Variables|/Script/Engine.PrimitiveComponent|SetbGenerateOverlapEvents (.Value (Utilities|Map|Find (Variables|Default|GetHitboxs) _array_element)) false)
      (else
        (Development|PrintString "没有找到这个Hitbox，请检查是否在Handle里注册了")))))

(event Custom|EnableHitbox
  (params (HitboxNames :type Array%20of%20Strings))
  (for _array_element HitboxNames
    (if (.ReturnValue (Utilities|Map|Find (Variables|Default|GetHitboxs) _array_element))
      (Variables|/Script/Engine.PrimitiveComponent|SetbGenerateOverlapEvents (.Value (Utilities|Map|Find (Variables|Default|GetHitboxs) _array_element)) true)
      (else
        (Development|PrintString "没有找到这个Hitbox，请检查是否在Handle里注册了")))))