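; BPC_HeadUI is a bot component that controls a temporary head UI and turns it to face the player camera.
; ShowUI enables the per-tick facing update, fires the OnHeadUIDrawChange dispatcher and sets a timer to call HideUI after ten seconds.
; HideUI fires the dispatcher with false, then waits briefly before clearing Draw and stopping the rotation updates.
; FaceCamera billboards by mirroring the camera rotation, with negated pitch and flipped yaw.
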(event Custom|ShowUI
  (Variables|Default|SetUpdateDir true)
  (if (Variables|Default|GetDraw)
    _
    (else
      (Variables|Default|SetDraw true)
      (Default|CallOnHeadUIDrawChange true)))
  (Utilities|Time|SetTimerbyEvent (delegate Custom|HideUI) 1e+01))

(event Custom|HideUI
  (if (Variables|Default|GetDraw)
    (Default|CallOnHeadUIDrawChange false)
    (Utilities|FlowControl|Delay 0.3)
    (Variables|Default|SetDraw false)
    (Variables|Default|SetUpdateDir false)))

(event EventBeginPlay)

(event EventTick
  (params (DeltaSeconds :type Float%20%28single-precision%29))
  (if (Variables|Default|GetUpdateDir)
    (CallFunction|FaceCamera)))

(fn FaceCamera
  (bind _returnvalue (Game|GetPlayerCameraManager 0))
  (bind _returnvalue_2 (Camera|GetCameraRotation _returnvalue))
  (bind (_roll _pitch _yaw) (Math|Rotator|BreakRotator _returnvalue_2))
  (Transformation|SetWorldRotation (Math|Rotator|MakeRotator _roll (* _pitch -1.0) (+ _yaw 1.8e+02)) false false))