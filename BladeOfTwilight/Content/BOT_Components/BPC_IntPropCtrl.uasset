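; Actor component that stores and manages integer properties for its owner, in a map from property type to a struct holding current, min and max values.
; GetPropVal looks up a property and logs when the map is empty or the key is missing.
; AddPropVal applies a delta clamped to that property's range, writes it back through SetUpProps, then calls OnPropValModify with the updated struct.
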(event EventBeginPlay)

(event EventTick
  (params (DeltaSeconds :type Float%20%28single-precision%29)))

(fn GetPropVal
  (params (PropType :type ChIntPropType%20Enum :default "NewEnumerator0"))
  (bind _chintprops (Variables|Default|GetChIntProps))
  (bind (_value _returnvalue) (Utilities|Map|Find _chintprops PropType))
  (if (Utilities|Map|IsEmpty _chintprops)
    (Utilities|String|LogString "属性集为空！")
    (elif _returnvalue
      (return _value true)
      (else
        (Utilities|String|LogString "没有找到对应的属性值！"))))
  (return "" false))

(fn AddPropVal
  (params (PropType :type ChIntPropType%20Enum :default "NewEnumerator0") (AddVal :type Integer))
  (bind (_propinfo _found) (CallFunction|GetPropVal PropType))
  (bind (_currentval _maxval _minval) (Utilities|Struct|BreakChIntProperty _propinfo))
  (if _found
    (bind _structout (Utilities|Struct|SetmembersinChIntProperty _propinfo (Math|Integer|Clamp(Integer) (+ _currentval AddVal) _minval _maxval)))
    (CallFunction|SetUpProps PropType _structout)
    (Default|CallOnPropValModify PropType _structout)
    (return)
    (else
      (Utilities|String|LogString "没有找到要设置的属性值"))))

(fn SetUpProps
  (params (PropType :type ChIntPropType%20Enum%20%28by%20ref%29 :default "NewEnumerator0") (PropInfo :type Ch%20Int%20Property%20Structure%20%28by%20ref%29))
  (Utilities|Map|Add (Variables|Default|GetChIntProps) PropType PropInfo))