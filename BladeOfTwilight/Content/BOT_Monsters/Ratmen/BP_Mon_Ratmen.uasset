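; Ratman monster character that fights with left, right and head weapon hitboxes attached to mesh sockets.
; On begin play it caches its anim blueprint and overhead bar widget, then fills the bars from the integer property component and updates them on change.
; Damage runs the parent logic, then plays a left or right hit montage section if still alive.
; Death triggers the death animation and hides the head UI, whose draw changes animate the bar.
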(event OnPropValModify(BPC_IntPropCtrl)
  (params (PropTrype :type ChIntPropType%20Enum :default "NewEnumerator13") (PropInfo :type Ch%20Int%20Property%20Structure))
  (Default|UpdateBar (stale EventBeginPlay _output_get) PropTrype PropInfo))

(event OnHeadUIDrawChange(BPI_HeadUI)
  (params (Draw :type Boolean))
  (bind _headui (Variables|Default|GetHeadUI))
  (bind _showbar (Variables|/Game/BOT_UI/UI_MonPropBar_Normal.UI_MonPropBar_Normal_C|GetShowBar _headui))
  (if Draw
    (UserInterface|Animation|PlayAnimation _headui _showbar 0.0 1 "Forward" 1.0 false)
    (else
      (UserInterface|Animation|PlayAnimation _headui _showbar 0.0 1 "Reverse" 1.0 false))))

(event EventTick
  (params (DeltaSeconds :type Float%20%28single-precision%29))
  (|CallParentFunction DeltaSeconds))

(event EventBeginPlay
  (bind _bpc_intpropctrl (Variables|Default|GetBPC_IntPropCtrl))
  (|CallParentFunction)
  (bind _asanim_bp_mon_ratmen (Utilities|Casting|CastToAnimBP_Mon_Ratmen (Components|SkeletalMesh|GetAnimInstance (Variables|Character|GetMesh))))
  (Variables|Default|SetAnimBP _asanim_bp_mon_ratmen)
  (bind _asui_mon_prop_bar_normal (Utilities|Casting|CastToUI_MonPropBar_Normal (UserInterface|GetUserWidgetObject (Variables|Default|GetBPI_HeadUI))))
  (bind _output_get (Variables|Default|SetHeadUI _asui_mon_prop_bar_normal))
  (for _array_element (Variables|/Game/BOT_Components/BPC_IntPropCtrl.BPC_IntPropCtrl_C|GetChIntPropsList _bpc_intpropctrl)
    (Default|UpdateBar _output_get _array_element (.PropInfo (Default|GetPropVal _bpc_intpropctrl _array_element)))))

(event EventOnDeath
  (|CallParentFunction)
  (Default|ToDeath (Variables|Default|GetAnimBP))
  (Default|HideUI (Variables|Default|GetBPI_HeadUI)))

(fn ConstructionScript
  (bind _mesh (Variables|Character|GetMesh))
  (bind _weapon_head (Variables|Default|GetWeapon_Head))
  (Transformation|AttachComponentToComponent (Variables|Default|GetWeapon_L) _mesh "Weapon_L_Socket" "KeepRelative" "KeepRelative" "KeepRelative" true)
  (Transformation|AttachComponentToComponent (Variables|Default|GetWeapon_R) _mesh "Weapon_R_Socket" "KeepRelative" "KeepRelative" "KeepRelative" true)
  (Transformation|AttachComponentToComponent _weapon_head _mesh "Weapon_Head_Socket" "KeepRelative" "KeepRelative" "KeepRelative" true)
  (Default|AddHitbox (Variables|Default|GetHitboxHandle) (Utilities|Array|MakeArray (Variables|Default|GetWeapon_L) (Variables|Default|GetWeapon_R) _weapon_head)))

(fn TryApplyDamage
  (params (DamageVar :type Integer) (AttackDir :type AttackDir%20Enum :default "NewEnumerator2"))
  (|CallParentFunction DamageVar "NewEnumerator0")
  (bind _alived (Default|IsAlived (Variables|Default|GetBPC_IntPropCtrl)))
  (if _alived
    (switch Utilities|FlowControl|Switch|SwitchonAttackDir AttackDir
      (:NewEnumerator0
        (Animation|PlayAnimMontage "/Game/BOT_AnimBP/Monsters/Ratmen/OnHit_Ratmen.OnHit_Ratmen" 1.0 "OnHit_L"))
      (:NewEnumerator1
        (Animation|PlayAnimMontage "/Game/BOT_AnimBP/Monsters/Ratmen/OnHit_Ratmen.OnHit_Ratmen" 1.0 "OnHit_R")))
    (return false)))