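; BP_BOT_Monster is a bot monster with a property bar and a death animation.
; The BPCIntPropCtrl component holds its properties, and TryApplyDamage adds the damage value to one of them, always returning false.
; Each Tick rotates the bar toward the player camera and polls the component's alive state, playing the Death_Ratmen montage once through DoOnce when the monster is no longer alive.
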(event EventTick
  (params (DeltaSeconds :type Float%20%28single-precision%29))
  (CallFunction|PropBarFaceCamera (Variables|Default|GetPropBar))
  (bind _alived (Default|IsAlived (Variables|Default|GetBPC_IntPropCtrl)))
  (if (not _alived)
    (Utilities|FlowControl|DoOnce false
      (:Completed
        (Animation|Montage|PlayMontage (Variables|Character|GetMesh) "/Game/BOT_AnimBP/Monsters/Ratmen/Death_Ratmen.Death_Ratmen" 1.0 0.0 "Death")))))

(fn ConstructionScript)

(fn TryApplyDamage
  (params (DamageVar :type Integer))
  (Default|AddPropVal (Variables|Default|GetBPC_IntPropCtrl) "NewEnumerator0" DamageVar)
  (return false))

(fn PropBarFaceCamera
  (params (Bar :type Widget%20Component%20Object%20Reference))
  (Transformation|SetWorldRotation Bar (Math|Rotator|FindLookatRotation (Transformation|GetWorldLocation Bar) (Camera|GetCameraLocation (Game|GetPlayerCameraManager 0))) false false))